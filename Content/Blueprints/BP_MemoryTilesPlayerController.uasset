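; Player controller for the Memory Tiles game that owns and drives the in-game HUD.
; On BeginPlay it creates the BP_GameHUD widget and adds it to the viewport.
; Custom events forward calls to that widget to show the success or fail screen and to update the remaining moves text.
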(event EventBeginPlay
  (bind _returnvalue (UserInterface|CreateWidget "/Game/Blueprints/BP_GameHUD.BP_GameHUD_C" self))
  (bind _output_get (Variables|Default|SetGameHUD _returnvalue))
  (UserInterface|Viewport|AddtoViewport _output_get 0))

(event EventShowGameFailHUD
  (Class|GameHUD|ShowGameFailScreen (Variables|Default|GetGameHUD)))

(event EventShowGameSuccessHUD
  (Class|GameHUD|ShowGameSuccessScreen (Variables|Default|GetGameHUD)))

(event EventUpdateRemainMovesText
  (params (RemainMovesCount :type Integer))
  (bind _gamehud (Variables|Default|GetGameHUD))
  (Utilities|IsValid _gamehud
    (:Is%20Valid
      (Default|OnUpdateMoves _gamehud (Utilities|String|ToString(Integer) RemainMovesCount)))))

(fn ConstructionScript)